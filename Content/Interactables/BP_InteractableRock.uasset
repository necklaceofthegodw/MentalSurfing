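; BP_InteractableRock is a rock actor that shows a name widget while it is being interacted with.
; The construction script applies the RockMesh variable to its static mesh component.
; InteractStarted unhides the widget component and passes the actor's display name to its WBP_Interaction widget, and InteractEnded hides it again.
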(event `/Game/Interactables/BPI_Interactable.InteractStarted`
  (`self.ShowInteractionWidget` true)
  (bind _aswbp_interaction (cast `/Game/Interactables/WBP_Interaction` (`WidgetComponent.GetUserWidgetObject` (`self.Widget`))))
  (`/Game/Interactables/WBP_Interaction.SetRockName` _aswbp_interaction (`KismetSystemLibrary.GetDisplayName` self)))

(event `/Game/Interactables/BPI_Interactable.InteractEnded`
  (`self.ShowInteractionWidget` false))

(fn `ShowInteractionWidget`
  (params (IsShown :type Boolean))
  (`SceneComponent.SetHiddenInGame` (`self.Widget`) (not IsShown) false))

(fn `UserConstructionScript`
  (`StaticMeshComponent.SetStaticMesh` (`self.StaticMesh`) (`self.RockMesh`)))